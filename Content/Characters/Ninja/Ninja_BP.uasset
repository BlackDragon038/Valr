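; Ninja character Blueprint for a fighting game that applies saved color customization to its skeletal mesh at spawn.
; On BeginPlay it casts the game instance to FightingGameInstance_BP and reads the Ninja color settings for headgear, two armor parts and two specials.
; It creates a dynamic material instance on each matching mesh material slot and sets that slot's color vector parameter.
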(event EventBeginPlay
  (bind _skeletalmesh (Variables|Default|GetSkeletalMesh))
  (bind _asfighting_game_instance_bp (Utilities|Casting|CastToFightingGameInstance_BP (Game|GetGameInstance)))
  (bind _returnvalue (Rendering|Material|CreateDynamicMaterialInstance _skeletalmesh 0 0 "None" :!class /Script/Engine.PrimitiveComponent))
  (Rendering|Material|SetVectorParameterValue _returnvalue "Headgear" (Utilities|Struct|MakeLinearColor (.R (Utilities|Struct|BreakColorData (.Headgear (Utilities|Struct|BreakCharacterColorData (Variables|/Script/Valr.FightingGameInstance|GetNinja _asfighting_game_instance_bp))))) (.G (Utilities|Struct|BreakColorData (.Headgear (Utilities|Struct|BreakCharacterColorData (Variables|/Script/Valr.FightingGameInstance|GetNinja _asfighting_game_instance_bp))))) (.B (Utilities|Struct|BreakColorData (.Headgear (Utilities|Struct|BreakCharacterColorData (Variables|/Script/Valr.FightingGameInstance|GetNinja _asfighting_game_instance_bp))))) 0.0) :!class /Script/Engine.MaterialInstanceDynamic)
  (bind _returnvalue_2 (Rendering|Material|CreateDynamicMaterialInstance _skeletalmesh 1 0 "None" :!class /Script/Engine.PrimitiveComponent))
  (Rendering|Material|SetVectorParameterValue _returnvalue_2 "Armor_1" (Utilities|Struct|MakeLinearColor (.R (Utilities|Struct|BreakColorData (.Armor_1 (Utilities|Struct|BreakCharacterColorData (Variables|/Script/Valr.FightingGameInstance|GetNinja _asfighting_game_instance_bp))))) (.G (Utilities|Struct|BreakColorData (.Armor_1 (Utilities|Struct|BreakCharacterColorData (Variables|/Script/Valr.FightingGameInstance|GetNinja _asfighting_game_instance_bp))))) (.B (Utilities|Struct|BreakColorData (.Armor_1 (Utilities|Struct|BreakCharacterColorData (Variables|/Script/Valr.FightingGameInstance|GetNinja _asfighting_game_instance_bp))))) 0.0) :!class /Script/Engine.MaterialInstanceDynamic)
  (bind _returnvalue_3 (Rendering|Material|CreateDynamicMaterialInstance _skeletalmesh 5 0 "None" :!class /Script/Engine.PrimitiveComponent))
  (Rendering|Material|SetVectorParameterValue _returnvalue_3 "Armor_2" (Utilities|Struct|MakeLinearColor (.R (Utilities|Struct|BreakColorData (.Armor_2 (Utilities|Struct|BreakCharacterColorData (Variables|/Script/Valr.FightingGameInstance|GetNinja _asfighting_game_instance_bp))))) (.G (Utilities|Struct|BreakColorData (.Armor_2 (Utilities|Struct|BreakCharacterColorData (Variables|/Script/Valr.FightingGameInstance|GetNinja _asfighting_game_instance_bp))))) (.B (Utilities|Struct|BreakColorData (.Armor_2 (Utilities|Struct|BreakCharacterColorData (Variables|/Script/Valr.FightingGameInstance|GetNinja _asfighting_game_instance_bp))))) 0.0) :!class /Script/Engine.MaterialInstanceDynamic)
  (bind _returnvalue_4 (Rendering|Material|CreateDynamicMaterialInstance _skeletalmesh 3 0 "None" :!class /Script/Engine.PrimitiveComponent))
  (Rendering|Material|SetVectorParameterValue _returnvalue_4 "Special_1" (Utilities|Struct|MakeLinearColor (.R (Utilities|Struct|BreakColorData (.Special_1 (Utilities|Struct|BreakCharacterColorData (Variables|/Script/Valr.FightingGameInstance|GetNinja _asfighting_game_instance_bp))))) (.G (Utilities|Struct|BreakColorData (.Special_1 (Utilities|Struct|BreakCharacterColorData (Variables|/Script/Valr.FightingGameInstance|GetNinja _asfighting_game_instance_bp))))) (.B (Utilities|Struct|BreakColorData (.Special_1 (Utilities|Struct|BreakCharacterColorData (Variables|/Script/Valr.FightingGameInstance|GetNinja _asfighting_game_instance_bp))))) 0.0) :!class /Script/Engine.MaterialInstanceDynamic)
  (bind _returnvalue_5 (Rendering|Material|CreateDynamicMaterialInstance _skeletalmesh 6 0 "None" :!class /Script/Engine.PrimitiveComponent))
  (Rendering|Material|SetVectorParameterValue _returnvalue_5 "Special_2" (Utilities|Struct|MakeLinearColor (.R (Utilities|Struct|BreakColorData (.Special_2 (Utilities|Struct|BreakCharacterColorData (Variables|/Script/Valr.FightingGameInstance|GetNinja _asfighting_game_instance_bp))))) (.G (Utilities|Struct|BreakColorData (.Special_2 (Utilities|Struct|BreakCharacterColorData (Variables|/Script/Valr.FightingGameInstance|GetNinja _asfighting_game_instance_bp))))) (.B (Utilities|Struct|BreakColorData (.Special_2 (Utilities|Struct|BreakCharacterColorData (Variables|/Script/Valr.FightingGameInstance|GetNinja _asfighting_game_instance_bp))))) 0.0) :!class /Script/Engine.MaterialInstanceDynamic))

(event Collision|EventActorBeginOverlap
  (params (OtherActor :type Actor%20Object%20Reference)))

(event EventTick
  (params (DeltaSeconds :type Float%20%28single-precision%29)))

(fn ConstructionScript)